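; BP_Arrow is an arrow projectile that sticks into what it hits and can then be picked up by the player.
; Overlaps on the arrow component feed HandleOverlap, which branches on the arrow's state.
; In the air, hitting anything but the player sets it to On Ground, nudges it forward from the hit point and attaches it to that actor.
; On the ground, a FirstPersonCharacter overlap adds one arrow and destroys it.
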(event OnComponentBeginOverlap(Arrow)
  (params (OverlappedComponent :type Primitive%20Component%20Object%20Reference) (OtherActor :type Actor%20Object%20Reference) (OtherComp :type Primitive%20Component%20Object%20Reference) (OtherBodyIndex :type Integer) (bFromSweep :type Boolean) (SweepResult :type Hit%20Result%20Structure%20%28by%20ref%29))
  (CallFunction|HandleOverlap OtherActor SweepResult))

(event EventBeginPlay
  (Variables|Default|SetcurrentState "AS_None")
  (Class|Arrow|SetArrowMesh (Variables|Default|GetArrow)))

(fn ConstructionScript)

(fn HandleOverlap
  (params (otherActor :type Actor%20Object%20Reference) (hitResult :type Hit%20Result%20Structure))
  (switch Utilities|FlowControl|Switch|SwitchonArrowStateC (Variables|Default|GetcurrentState)
    (:AS_OnGround
      (bind _asfirst_person_character (Utilities|Casting|CastToFirstPersonCharacter otherActor))
      (Default|AddArrow _asfirst_person_character 1)
      (Actor|DestroyActor))
    (:AS_InAir
      (if (!= otherActor (Game|GetPlayerCharacter 0))
        (Class|Arrow|SetArrowStateC "AS_OnGround")
        (Transformation|SetActorLocation (+ (.location hitResult) (* (Transformation|GetActorForwardVector) 4e+01)) false true)
        (Transformation|AttachActorToActor otherActor "None" "KeepWorld" "KeepWorld" "KeepWorld" true)))))