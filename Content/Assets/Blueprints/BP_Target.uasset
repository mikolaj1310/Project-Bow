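; Archery target actor that awards points to the player when a BP_Arrow overlaps its Target mesh.
; On overlap it passes the arrow to HandleTargetOverlap, defined outside this file, then adds ScoreAmountC to the FirstPersonCharacter's score via IncrementScore.
; Disconnected leftover nodes hold a Blueprint version of ring scoring by the arrow tip's distance from center, plus trace and print debugging; none of it runs.
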(event OnComponentBeginOverlap(Target)
  (params (OverlappedComponent :type Primitive%20Component%20Object%20Reference) (OtherActor :type Actor%20Object%20Reference) (OtherComp :type Primitive%20Component%20Object%20Reference) (OtherBodyIndex :type Integer) (bFromSweep :type Boolean) (SweepResult :type Hit%20Result%20Structure%20%28by%20ref%29))
  (bind _asbp_arrow (Utilities|Casting|CastToBP_Arrow OtherActor))
  (Class|Target|HandleTargetOverlap _asbp_arrow)
  (bind _returnvalue (Actor|GetActorOfClass "/Game/FirstPersonBP/Blueprints/FirstPersonCharacter.FirstPersonCharacter_C"))
  (Default|IncrementScore _returnvalue (Math|Conversions|ToFloat(Integer) (Variables|Default|GetscoreAmountC))))

(event EventBeginPlay
  (Variables|Default|SettargetMesh (Variables|Default|GetTarget)))

(fn ConstructionScript)