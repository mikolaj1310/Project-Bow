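; BP_Bow is a bow weapon Blueprint that handles charging, firing and reloading arrows.
; While an arrow is valid, BeginCharge and EndCharge play and reverse a timeline whose updates drive ChargeAmountC.
; Fire calls FireArrowC, clears the arrow reference, then stops and rewinds the timeline through StopCharge.
; Reload delegates to ReloadC; neither it nor FireArrowC is defined in these graphs.
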(event Custom|BeginCharge
  (Variables|Default|GetarrowC
    (:then
      (bind _chargeamount (Timeline|ChargeTimeline Play)
        (:Update
          (Variables|Default|SetchargeAmountC _chargeamount))))
    (:else)))

(event Custom|StopCharge
  (Utilities|FlowControl|Sequence
    (:then_0
      (bind _chargeamount (Timeline|ChargeTimeline Stop)
        (:Update
          (Variables|Default|SetchargeAmountC _chargeamount))))
    (:then_1
      (Timeline|ChargeTimeline SetNewTime))))

(event Custom|EndCharge
  (Variables|Default|GetarrowC
    (:then
      (bind _chargeamount (Timeline|ChargeTimeline Reverse)
        (:Update
          (Variables|Default|SetchargeAmountC _chargeamount))))
    (:else)))

(event Custom|Fire
  (Class|Bow|FireArrowC)
  (Variables|Default|SetarrowC 0)
  (CallFunction|StopCharge))

(event Custom|Reload
  (Class|Bow|ReloadC))

(fn ConstructionScript)